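; Interactible record player actor that toggles on and off with a switch sound, spinning up and winding down gradually.
; Interact sets a goal rotation rate, which Tick eases toward at constant speed to accumulate record rotation.
; The ratio of current to max rate drives music pitch, plus music and noise volume through a curve, mimicking a real turntable.
; A DoOnce pauses both audio components once it stops.
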(event `self.ReceiveBeginPlay`
  (bind _music (`self.Music`))
  (`parent.ReceiveBeginPlay`)
  ;[0.2 0.16 0.16] Bind Update Playback Percent event, then activate the audio
  (add `AudioComponent.OnAudioPlaybackPercent` _music (delegate `UpdateMusic`))
  (`ActorComponent.Activate` _music false))

(event `UpdateMusic`
  (params (PlayingSoundWave :type "SoundWave Object Reference") (PlaybackPercent :type "Float (single-precision)"))
  ;[0.2 0.16 0.16] Bind Update Playback Percent event, then activate the audio
)

(event `self.ReceiveTick`
  (params (DeltaSeconds :type "Float (single-precision)"))
  (bind _music (`self.Music`))
  (`parent.ReceiveTick` DeltaSeconds)
  ;[0.2 0.16 0.16] Is the Record Player on and/or spinning?
  (if (or (`self.bIsOn`) (> (`self.RotationRate`) 0.0))
    (set `self.PlaybackPercentage` (stale `UpdateMusic` PlaybackPercent))
    ;[0.2 0.16 0.16] Pause/play audio
    (`|ExecutionSequence`
      (:`then_0`
        (`AudioComponent.SetPaused` _music false)
        (`AudioComponent.SetPaused` (`self.Noise`) false)
        ;[0.2 0.16 0.16] Set Record rotation
        (set `self.RotationRate` (`KismetMathLibrary.FInterpTo_Constant` (`self.RotationRate`) (`self.GoalRotationRate`) (`GameplayStatics.GetWorldDeltaSeconds`) 64.0))
        (set `self.Rotation` (+ (`self.Rotation`) (* (`self.RotationRate`) (`GameplayStatics.GetWorldDeltaSeconds`))))
        ;[0.2 0.16 0.16] Set pitch/tempo
        (`AudioComponent.SetPitchMultiplier` (`self.Music`) (/ (`self.RotationRate`) (`self.MaxRotationRate`)))
        ;[0.2 0.16 0.16] Set volume
        (`AudioComponent.SetVolumeMultiplier` (`self.Music`) (`CurveFloat.GetFloatValue` (`self.VolumeCurve`) (/ (`self.RotationRate`) (`self.MaxRotationRate`))))
        (`AudioComponent.SetVolumeMultiplier` (`self.Noise`) (`CurveFloat.GetFloatValue` (`self.VolumeCurve`) (/ (`self.RotationRate`) (`self.MaxRotationRate`)))))
      (:`then_1`
        (goto _label :!via `Reset`)))
    (else
      (`/Engine/EditorBlueprintResources/StandardMacros.DoOnce` false :!label _label
        (:`Completed`
          (`AudioComponent.SetPaused` _music true)
          (`AudioComponent.SetPaused` (`self.Noise`) true))))))

(fn `Interact`
  (params (Component :type "BoxComponent Object Reference"))
  (`parent.Interact` Component)
  ;[0.2 0.16 0.16] Toggle the Record Player on/off
  (set `self.bIsOn` (not (`self.bIsOn`)))
  ;[0.2 0.16 0.16] Set Goal Rotation Rate
  (set `self.GoalRotationRate` (`KismetMathLibrary.SelectFloat` (`self.MaxRotationRate`) 0.0 (`self.bIsOn`)))
  ;[0.2 0.16 0.16] Play Switch audio
  (`GameplayStatics.PlaySoundAtLocation` "/Game/AudioExperiments/Sounds/S_RecordPlayer_Switch.S_RecordPlayer_Switch" (`SceneComponent.GetSocketLocation` (`self.SkeletalMesh`) "switch_jnt") (struct) 1.0 1.0 0.0 null null null null))

(fn `UserConstructionScript`
  (`parent.UserConstructionScript`))