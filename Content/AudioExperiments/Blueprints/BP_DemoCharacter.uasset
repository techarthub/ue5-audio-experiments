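; First-person player character for the AudioExperiments demo, with half-scaled walk and look input and a cursor widget created at BeginPlay.
; Each tick a short camera line trace caches any BP_Interactible hit on a box component and toggles the cursor's Interaction flag.
; The Interact action passes that box to the interactible, so it can tell which collider was targeted.
; The cursor's Movement flag is true only while both move axes are zero, despite its name.
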(event `self.ReceiveBeginPlay`
  ;[0.2 0.16 0.16] HUD setup
  (bind _returnvalue (`|CreateWidget` "/Game/AudioExperiments/Blueprints/WBP_Cursor.WBP_Cursor_C"))
  (bind _output_get (set `self.WBP_Cursor` _returnvalue))
  (`UserWidget.AddToViewport` _output_get 0)
  (`self.AddControllerPitchInput` 15.0))

(event `self.ReceiveTick`
  (params (DeltaSeconds :type "Float (single-precision)"))
  ;[0.2 0.16 0.16] Checking for interactions
  (`self.CheckForInteractable `)
  (`self.CheckForMovement`))

(event `InputAxis|Move Forward/Backward`
  (params (AxisValue :type "Float (single-precision)"))
  ;[0.2 0.16 0.16] Movement
  (`self.AddMovementInput` (`self.GetActorForwardVector`) (* AxisValue 0.5)))

(event `InputAxis|Move Right/Left`
  (params (AxisValue :type "Float (single-precision)"))
  ;[0.2 0.16 0.16] Movement
  (`self.AddMovementInput` (`self.GetActorRightVector`) (* AxisValue 0.5)))

(event `InputAxis|Turn Right/Left`
  (params (AxisValue :type "Float (single-precision)"))
  ;[0.2 0.16 0.16] Camera control
  (`self.AddControllerYawInput` (* AxisValue 0.5)))

(event `InputAxis|Look Up/Down`
  (params (AxisValue :type "Float (single-precision)"))
  ;[0.2 0.16 0.16] Camera control
  (`self.AddControllerPitchInput` (* AxisValue 0.5)))

(event `InputAction|Interact`
  (params (Key :type "Key Structure"))
  (:`Pressed`
    ;[0.2 0.16 0.16] Interaction
    (bind _interactablecollider (`self.InteractableCollider`)
      (:`then`
        (`/Game/AudioExperiments/Blueprints/BP_Interactible.Interact` (`self.Interactable`) _interactablecollider))
      (:`else`))))

(fn `CheckForInteractable `
  (bind _firstpersoncamera (`self.FirstPersonCamera`))
  (bind _wbp_cursor (`self.WBP_Cursor`))
  (bind _returnvalue (`SceneComponent.K2_GetComponentLocation` _firstpersoncamera))
  (bind _outhit (`KismetSystemLibrary.LineTraceSingle` _returnvalue (+ _returnvalue (* (`SceneComponent.GetForwardVector` _firstpersoncamera) 200.0)) "TraceTypeQuery1"))
  (bind _asbp_interactible (cast `/Game/AudioExperiments/Blueprints/BP_Interactible` (`.HitActor` (`GameplayStatics.BreakHitResult` _outhit)))
    (:`then`
      (bind _asbox_collision (cast `BoxComponent` (`.HitComponent` (`GameplayStatics.BreakHitResult` _outhit)))
        (:`then`
          (set `/Game/AudioExperiments/Blueprints/WBP_Cursor.Interaction` true _wbp_cursor)
          (set `self.Interactable` _asbp_interactible)
          (set `self.InteractableCollider` _asbox_collision))
        (:`CastFailed`
          (set `/Game/AudioExperiments/Blueprints/WBP_Cursor.Interaction` false _wbp_cursor :!label _label)
          (set `self.Interactable` null)
          (set `self.InteractableCollider` null))))
    (:`CastFailed`
      (goto _label))))

(fn `CheckForMovement`
  (bind _wbp_cursor (`self.WBP_Cursor`))
  (if (and (== (`self.GetInputAxisValue`) 0.0) (== (`self.GetInputAxisValue`) 0.0))
    (set `/Game/AudioExperiments/Blueprints/WBP_Cursor.Movement` true _wbp_cursor)
    (else
      (set `/Game/AudioExperiments/Blueprints/WBP_Cursor.Movement` false _wbp_cursor))))

(fn `UserConstructionScript`)