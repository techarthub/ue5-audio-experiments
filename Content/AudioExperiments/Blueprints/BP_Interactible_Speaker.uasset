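; Interactible speaker with a five-position slider that switches between variants of a Waltz in A Minor track.
; Interact reads the last character of the hit collider's name, steps Stage one notch toward it, and disables the collider at the new position.
; Each switch swaps the sound cue, resumes it at the same relative playback percentage, and plays a switch sound.
; Tick eases SliderPosition toward the stage's target.
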(event `self.ReceiveBeginPlay`
  (bind _music (`self.Music`))
  (`parent.ReceiveBeginPlay`)
  ;[0.2 0.16 0.16] Bind Update Playback Percent event, then activate the audio
  (add `AudioComponent.OnAudioPlaybackPercent` _music (delegate `UpdateMusic`))
  (`ActorComponent.Activate` _music false))

(event `UpdateMusic`
  (params (PlayingSoundWave :type "SoundWave Object Reference") (PlaybackPercent :type "Float (single-precision)"))
  ;[0.2 0.16 0.16] Bind Update Playback Percent event, then activate the audio
  (set `self.Percentage` PlaybackPercent))

(event `self.ReceiveTick`
  (params (DeltaSeconds :type "Float (single-precision)"))
  (`parent.ReceiveTick` DeltaSeconds)
  ;[0.2 0.16 0.16] Does the Slider need to move?
  (if (!= (`self.SliderPosition`) (`self.SliderTarget`))
    ;[0.2 0.16 0.16] Interp to new Slider Position
    (set `self.SliderPosition` (`KismetMathLibrary.FInterpTo` (`self.SliderPosition`) (`self.SliderTarget`) (`GameplayStatics.GetWorldDeltaSeconds`) 16.0))))

(fn `Interact`
  (params (Component :type "BoxComponent Object Reference"))
  (bind _returnvalue (`KismetSystemLibrary.GetDisplayName` Component))
  (bind _stage (`self.Stage`))
  (bind _returnvalue_2 (select `int` (`self.Stage`) :`0` "/Game/AudioExperiments/Sounds/S_WaltzInAMinor_75_Cue.S_WaltzInAMinor_75_Cue" :`1` "/Game/AudioExperiments/Sounds/S_WaltzInAMinor_50_Cue.S_WaltzInAMinor_50_Cue" :`2` "/Game/AudioExperiments/Sounds/S_WaltzInAMinor_100_Cue.S_WaltzInAMinor_100_Cue" :`3` "/Game/AudioExperiments/Sounds/S_WaltzInAMinor_125_Cue.S_WaltzInAMinor_125_Cue" :`4` "/Game/AudioExperiments/Sounds/S_WaltzInAMinor_175_Cue.S_WaltzInAMinor_175_Cue" :!type "SoundBase Object Reference"))
  (bind _returnvalue_3 (`KismetStringLibrary.Conv_StringToInt` (`KismetStringLibrary.RightChop` _returnvalue (- (`KismetStringLibrary.Len` _returnvalue) 1))))
  (`parent.Interact` Component)
  ;[0.2 0.16 0.16] Renable the collider for the Slider's previous position
  (`PrimitiveComponent.SetCollisionEnabled` (select `int` (`self.Stage`) :`0` (`self.Collider0`) :`1` (`self.Collider1`) :`2` (`self.Collider2`) :`3` (`self.Collider3`) :`4` (`self.Collider4`) :!type "PrimitiveComponent Object Reference") "QueryOnly")
  ;[0.2 0.16 0.16] Set the current state of the Slider
  (if (!= _returnvalue_3 _stage)
    (set `self.Stage` (select `bool` (> _stage _returnvalue_3) :`false` (+ _stage 1) :`true` (+ _stage -1)))
    ;[0.2 0.16 0.16] Disable the collider for the Slider's current position
    (`PrimitiveComponent.SetCollisionEnabled` (select `int` (`self.Stage`) :`0` (`self.Collider0`) :`1` (`self.Collider1`) :`2` (`self.Collider2`) :`3` (`self.Collider3`) :`4` (`self.Collider4`) :!type "PrimitiveComponent Object Reference") "NoCollision")
    ;[0.2 0.16 0.16] Set Slider interp target
    (set `self.SliderTarget` (select `int` (`self.Stage`) :`0` 13.2 :`1` 6.6 :`2` 0.0 :`3` -6.6 :`4` -13.2))
    ;[0.2 0.16 0.16] Set the appropriate sound cue, and play it from the same relative position as the previous one.
    (`AudioComponent.SetSound` (`self.Music`) _returnvalue_2)
    (`AudioComponent.Play` (`self.Music`) (* (`self.Percentage`) (`SoundBase.Duration` _returnvalue_2)))
    ;[0.2 0.16 0.16] Play Switch audio
    (`GameplayStatics.PlaySoundAtLocation` "/Game/AudioExperiments/Sounds/S_Speaker_Switch_Cue.S_Speaker_Switch_Cue" (`SceneComponent.GetSocketLocation` (`self.SkeletalMesh`) "switch_jnt") (struct) 1.0 1.0 0.0 null null null null)))

(fn `UserConstructionScript`
  (`parent.UserConstructionScript`))